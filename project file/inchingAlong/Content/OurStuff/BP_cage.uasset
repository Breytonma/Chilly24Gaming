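; BP_cage is a cage that reacts when a lever event carries an ID matching its CageID.
; On BeginPlay it binds to the CageIndicator dispatcher on the player's BP_ThirdPersonCharacter, so the character relays lever IDs to the cage.
; On a match, it switches the Indicator to a green material and instantly shifts Lifters upward while applying a scale delta, with no animation.
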(event `self.ReceiveBeginPlay`
  (bind _asbp_third_person_character (cast `/Game/OurStuff/BP_ThirdPersonCharacter` (`GameplayStatics.GetPlayerCharacter` 0)))
  (add `/Game/OurStuff/BP_ThirdPersonCharacter.cageIndicator` _asbp_third_person_character (delegate `cageIndicator_Event`)))

(event `cageIndicator_Event`
  (params (leverIDs :type Integer))
  (if (== leverIDs (`self.cageID`))
    (`PrimitiveComponent.SetMaterial` (`self.indicator`) 0 "/Game/OurStuff/materials/MAT_basicGreen.MAT_basicGreen")
    (`SceneComponent.K2_AddWorldTransform` (`self.lifters`) (`KismetMathLibrary.MakeTransform` (0.0 0.0 400.0) (struct) (0.5 0.5 0.5)) false false)))

(fn `UserConstructionScript`)