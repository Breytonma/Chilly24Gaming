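; Enemy AI character, apparently an isopod, that moves on command from the player character and can jump across gaps.
; On BeginPlay it binds to the player's AI move call to run AIMoveTo, while player shouts alternately set and clear the "hasSeenPlayer?" Blackboard key.
; Jumps suspend gravity and lerp location via a timeline, flagging "atJump" until finished.
; Overlapping the hammer only prints a death message.
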(event `self.ReceiveBeginPlay`
  (bind _asbp_third_person_character (cast `/Game/OurStuff/BP_ThirdPersonCharacter` (`GameplayStatics.GetPlayerCharacter` 0)))
  (bind _output_get (set `self.As BP Third Person Character` _asbp_third_person_character))
  (add `/Game/OurStuff/BP_ThirdPersonCharacter.aiMoveCall` _output_get (delegate `AiMoveCall`)))

(event `AiMoveCall`
  (params (worldLocation :type "Vector Structure"))
  (`|AIMoveTo` self worldLocation null))

(event `/Game/OurStuff/AI_stuff/BPI_EnemyAI.playerShout`
  (`/Engine/EditorBlueprintResources/StandardMacros.FlipFlop`
    (:`A`
      (`BlackboardComponent.SetValueAsBool` (`AIBlueprintHelperLibrary.GetBlackboard` (`AIBlueprintHelperLibrary.GetAIController` self)) "hasSeenPlayer?" true))
    (:`B`
      (`BlackboardComponent.SetValueAsBool` (`AIBlueprintHelperLibrary.GetBlackboard` (`AIBlueprintHelperLibrary.GetAIController` self)) "hasSeenPlayer?" false))))

(event `self.ReceiveActorBeginOverlap`
  (params (OtherActor :type "Actor Object Reference"))
  (if (== OtherActor "/Game/OurStuff/ModelUploads/hammer/BP_hammer.BP_hammer")
    (`KismetSystemLibrary.PrintString` "ISOPOD DIED" true true (struct :`R` 1.0 :`G` 0.059196 :`A` 1.0) 10.0)))

(event `/Game/OurStuff/AI_stuff/BPI_EnemyAI.JumpToDestination`
  (params (Destination :type "Vector Structure"))
  (bind _charactermovement (`self.CharacterMovement`))
  (`BlackboardComponent.SetValueAsBool` (`AIBlueprintHelperLibrary.GetBlackboard` (`AIBlueprintHelperLibrary.GetAIController` self)) "atJump" true)
  (`PrimitiveComponent.SetEnableGravity` (`self.CapsuleComponent`) false)
  (set `CharacterMovementComponent.GravityScale` 0.0 _charactermovement)
  (`MovementComponent.StopMovementImmediately` _charactermovement)
  (bind (_direction _ai_gapper) (`Timeline|AI_cross` :!via `PlayFromStart`)
    (:`Update`
      (`self.K2_SetActorLocation` (`KismetMathLibrary.VLerp` (`self.K2_GetActorLocation`) (+ Destination (0.0 0.0 100.0)) _ai_gapper)))
    (:`Finished`
      (set `CharacterMovementComponent.GravityScale` 1.0 (`self.CharacterMovement`))
      (`PrimitiveComponent.SetEnableGravity` (`self.CapsuleComponent`) true)
      (`BlackboardComponent.SetValueAsBool` (`AIBlueprintHelperLibrary.GetBlackboard` (`AIBlueprintHelperLibrary.GetAIController` self)) "atJump" false))))

(fn `UserConstructionScript`)