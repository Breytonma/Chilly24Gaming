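; BP_lever is a one-shot lever that flips when the player character overlaps its Box.
; A DoOnce gate plays the RotateLever timeline, which lerps the Handle's relative rotation to swing it to the opposite tilt.
; When the timeline finishes, it calls CallCageIndicator with its LeverID on the BP_ThirdPersonCharacter cached at BeginPlay, then sets HasBeenFlipped.
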(event `self.ReceiveBeginPlay`
  (bind _asbp_third_person_character (cast `/Game/OurStuff/BP_ThirdPersonCharacter` (`GameplayStatics.GetPlayerCharacter` 0)))
  (set `self.As BP Third Person Character` _asbp_third_person_character))

(event `self.Box.OnComponentBeginOverlap`
  (params (OverlappedComponent :type "PrimitiveComponent Object Reference") (OtherActor :type "Actor Object Reference") (OtherComp :type "PrimitiveComponent Object Reference") (OtherBodyIndex :type Integer) (bFromSweep :type Boolean) (SweepResult :type "HitResult Structure (by ref)"))
  (if (== OtherActor (`GameplayStatics.GetPlayerCharacter` 0))
    (if true
      (`/Engine/EditorBlueprintResources/StandardMacros.DoOnce` false
        (:`Completed`
          (bind (_direction _newtrack_0) (`Timeline|RotateLever` :!via `PlayFromStart`)
            (:`Update`
              (`SceneComponent.K2_SetRelativeRotation` (`self.Handle`) (`KismetMathLibrary.RLerp` (struct :`Roll` 30.0) (struct :`Roll` -30.0) _newtrack_0) false false))
            (:`Finished`
              (`/Game/OurStuff/BP_ThirdPersonCharacter.cageIndicator` (`self.As BP Third Person Character`) (`self.leverID`))
              (set `self.hasBeenFlipped` true))))))))

(fn `UserConstructionScript`)