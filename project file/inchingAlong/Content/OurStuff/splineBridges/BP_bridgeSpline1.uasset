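; Spline bridge actor that lays cube spline meshes with collision along its spline in equal-length sections.
; The build runs in Tick with no guard, so it adds a new set of components every frame; the Construction Script is empty.
; Helper functions sample each section's endpoints and clamp tangents to the section length.
; Options derive section length from actor X scale or restrict the count to full-length pieces.
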(event `self.ReceiveTick`
  (params (DeltaSeconds :type "Float (single-precision)"))
  (bind _returnvalue_x (`KismetMathLibrary.BreakVector` (`self.GetActorScale3D`)))
  (bind _loop_index (`self.Loop Index`))
  (if (`self.allowScaling?`)
    (set `self.sectionLength` (* _returnvalue_x 100.0)))
  (if (`self.Must be Full Length Meshes?`)
    ;[1 1 1] Must Be full length members
    (for _index (range (`KismetMathLibrary.FTrunc` (/ (`SplineComponent.GetSplineLength` (`self.Spline`)) (`self.sectionLength`))))
      (set `self.Loop Index` _index)
      (bind _returnvalue (`AddComponent|NODE_AddSplineMeshComponent-3` :!label _label))
      (set `self.mesh` _returnvalue)
      (`StaticMeshComponent.SetStaticMesh` _returnvalue "/Game/starterStuff/StarterContent/Shapes/Shape_Cube.Shape_Cube")
      ;[1 1 1] Open mesh and look at gizmo
      (`SplineMeshComponent.SetForwardAxis` _returnvalue "X" true)
      (bind (_position _tangent) (`self.Get Start Pos/tangent` _loop_index))
      (bind (_position_2 _tangent_2) (`self.Get end Pos/tangent` _loop_index))
      (`SplineMeshComponent.SetStartAndEnd` _returnvalue _position _tangent _position_2 _tangent_2 true)
      (`PrimitiveComponent.SetCollisionEnabled` _returnvalue "QueryAndPhysics"))
    (else
      ;[1 1 1] Amount of Spline meshes
      (for _index_2 (range (+ (`KismetMathLibrary.FTrunc` (/ (`SplineComponent.GetSplineLength` (`self.Spline`)) (`self.sectionLength`))) 1))
        (set `self.Loop Index` _index_2)
        (goto _label)))))

(fn `Get end Pos/tangent`
  (params (index :type Integer))
  (returns (position :type "Vector Structure") (tangent :type "Vector Structure"))
  (bind _spline (`self.Spline`))
  (bind _returnvalue (* (+ index 1) (`self.sectionLength`)))
  ;[1 1 1] takes index and distance to get the piece at that location
  (return (`SplineComponent.GetLocationAtDistanceAlongSpline` _spline _returnvalue "Local") (`KismetMathLibrary.ClampVectorSize` (`SplineComponent.GetTangentAtDistanceAlongSpline` _spline _returnvalue "Local") 0.0 (`self.sectionLength`))))

(fn `Get Start Pos/tangent`
  (params (index :type Integer))
  (returns (position :type "Vector Structure") (tangent :type "Vector Structure"))
  (bind _spline (`self.Spline`))
  (bind _returnvalue (* index (`self.sectionLength`)))
  ;[1 1 1] takes index and distance to get the piece at that location
  (return (`SplineComponent.GetLocationAtDistanceAlongSpline` _spline _returnvalue "Local") (`KismetMathLibrary.ClampVectorSize` (`SplineComponent.GetTangentAtDistanceAlongSpline` _spline _returnvalue "Local") 0.0 (`self.sectionLength`))))

(fn `UserConstructionScript`)